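; BP_HPItem is a health item pickup that goes into the snowman player's inventory.
; On BeginPlay it fills its ItemInfo struct with itself and caches the BP_SnowMan player character.
; Any hit on its Sphere component, with no check on the other actor, adds ItemInfo to that inventory, refreshes it and destroys the pickup.
; UseAction is empty, and the logic adding AddHealth to the character's Energy is disconnected.
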(event `self.ReceiveBeginPlay`
  (setmembers `/Game/JWContents/BP/InventoryStructure` :`StructRef` (`self.ItemInfo`) :`Item` self)
  (bind _asbp_snow_man (cast `/Game/GameContents/BP_SnowMan` (`GameplayStatics.GetPlayerCharacter` 0)))
  (set `self.Character Reference` _asbp_snow_man))

(event `/Game/JWContents/BP/ActionInterface.UseAction`
  (params (NewParam :type Boolean))
  ;[1 1 1] 아이템 사용
)

(event `self.Sphere.OnComponentHit`
  (params (HitComponent :type "PrimitiveComponent Object Reference") (OtherActor :type "Actor Object Reference") (OtherComp :type "PrimitiveComponent Object Reference") (NormalImpulse :type "Vector Structure") (Hit :type "HitResult Structure (by ref)"))
  (bind _inventory (`/Game/GameContents/BP_SnowMan.Inventory` (`self.Character Reference`)))
  ;[1 1 1] 아이템 인벤토리 추가
  (`KismetArrayLibrary.Array_Add` (`/Game/JWContents/BP/BP_UIInventoryitem.Inventory` _inventory) (`self.ItemInfo`))
  (`/Game/JWContents/BP/BP_UIInventoryitem.RefreshInventory` _inventory)
  (`self.K2_DestroyActor`))

(fn `UserConstructionScript`)