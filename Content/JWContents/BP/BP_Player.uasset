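; BP_Player is a player-controlled Blueprint that moves from two input axes and enables input from player controller 0 on BeginPlay.
; The Horizon and Vertical axis events share one assignment that builds a Direction vector with zero Z.
; Tick normalizes Direction, scales it by Speed and delta time, and sets the new actor location directly without sweeping, so movement does no collision blocking.
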(event `self.ReceiveBeginPlay`
  (`self.EnableInput` (`GameplayStatics.GetPlayerController` 0)))

(event `InputAction|Jump`
  (params (Key :type "Key Structure")))

(event `InputAxis|Horizon`
  (params (AxisValue :type "Float (single-precision)"))
  (set `self.direction` (`KismetMathLibrary.MakeVector` (stale `InputAxis|Vertical` AxisValue) AxisValue) :!label _label))

(event `InputAxis|Vertical`
  (params (AxisValue :type "Float (single-precision)"))
  (goto _label))

(event `self.ReceiveTick`
  (params (DeltaSeconds :type "Float (single-precision)"))
  (`self.K2_SetActorLocation` (+ (* (* (`KismetMathLibrary.Normal` (`self.direction`)) (`self.speed`)) DeltaSeconds) (`self.K2_GetActorLocation`))))

(fn `UserConstructionScript`)