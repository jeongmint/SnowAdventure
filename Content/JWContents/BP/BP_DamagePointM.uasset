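; BP_DamagePointM is a short-lived damage point actor that drifts upward, stops, and then disappears.
; BeginPlay sets the direction to straight up and gives the actor a one-second lifespan.
; Tick moves it by direction, Speed and delta time, while a short Delay in the same chain zeroes Speed, so it hangs in place until destroyed.
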(event `self.ReceiveBeginPlay`
  ;[1 1 1] 데미지 포인트 이동하다 사라짐
  (set `self.Distriction` (`KismetMathLibrary.MakeVector` 0.0 0.0 1.0))
  (`self.SetLifeSpan` 1.0))

(event `self.ReceiveTick`
  (params (DeltaSeconds :type "Float (single-precision)"))
  (`self.K2_SetActorLocation` (+ (* (* (`self.Distriction`) (`self.Speed`)) DeltaSeconds) (`self.K2_GetActorLocation`)))
  ;[1 1 1] 데미지 포인트 멈춤
  (`KismetSystemLibrary.Delay` 0.2)
  (set `self.Speed` 0.0))

(fn `UserConstructionScript`)