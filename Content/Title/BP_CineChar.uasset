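; BP_CineChar is a title-folder character Blueprint, apparently for cinematics, that exposes two functions for spawning snow and ice effects.
; Iceball spawns a snow steam emitter and an Iceball actor at the Arrow1 component's transform to fire a snowball with a launch effect.
; Snowice spawns eight snowice emitter actors at the actor's own transform.
; The event graph and construction script are empty, so nothing in this Blueprint calls either function.
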(fn `iceball`
  ;[1 1 1] 발사 효과
  (`|SpawnActorFromClass` "/Game/JWContents/BP/EmitterSnowSteam.EmitterSnowSteam_C" (`SceneComponent.K2_GetComponentToWorld` (`self.Arrow1`)) "Undefined" "OverrideRootScale" null null)
  ;[1 1 1] 눈덩이 생성 발사
  (`|SpawnActorFromClass` "/Game/GameContents/Iceball.Iceball_C" (`SceneComponent.K2_GetComponentToWorld` (`self.Arrow1`)) "Undefined" "OverrideRootScale" null null))

(fn `snowice`
  (`|SpawnActorFromClass` "/Game/JWContents/BP/Emittersnowice.Emittersnowice_C" (`self.GetTransform`) "Undefined" "OverrideRootScale" null null)
  (`|SpawnActorFromClass` "/Game/JWContents/BP/Emittersnowice_2.Emittersnowice_2_C" (`self.GetTransform`) "Undefined" "OverrideRootScale" null null)
  (`|SpawnActorFromClass` "/Game/JWContents/BP/Emittersnowice_3.Emittersnowice_3_C" (`self.GetTransform`) "Undefined" "OverrideRootScale" null null)
  (`|SpawnActorFromClass` "/Game/JWContents/BP/Emittersnowice_4.Emittersnowice_4_C" (`self.GetTransform`) "Undefined" "OverrideRootScale" null null)
  (`|SpawnActorFromClass` "/Game/JWContents/BP/Emittersnowice_5.Emittersnowice_5_C" (`self.GetTransform`) "Undefined" "OverrideRootScale" null null)
  (`|SpawnActorFromClass` "/Game/JWContents/BP/Emittersnowice_6.Emittersnowice_6_C" (`self.GetTransform`) "Undefined" "OverrideRootScale" null null)
  (`|SpawnActorFromClass` "/Game/JWContents/BP/Emittersnowice_7.Emittersnowice_7_C" (`self.GetTransform`) "Undefined" "OverrideRootScale" null null)
  (`|SpawnActorFromClass` "/Game/JWContents/BP/Emittersnowice_8.Emittersnowice_8_C" (`self.GetTransform`) "Undefined" "OverrideRootScale" null null))

(fn `UserConstructionScript`)