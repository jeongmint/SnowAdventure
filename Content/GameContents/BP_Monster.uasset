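; BP_Monster is an enemy that homes in on BP_SnowMan and fires BP_MonsterBullet.
; BeginPlay finds the target, sets a looping timer, spawns a bullet at its own transform and caches the Energybar1 widget.
; Tick moves it with sweep along a direction that FindDirection refreshes toward the target every frame.
; AnyDamage drains Energy, updates the bar as a fraction of NormEnergy and destroys the actor at zero.
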(event `self.ReceiveBeginPlay`
  (bind _returnvalue (`GameplayStatics.GetActorOfClass` "/Game/GameContents/BP_SnowMan.BP_SnowMan_C"))
  (set `self.Target` _returnvalue)
  ;[1 1 1] 찾은 벡터 방향으로
  (`self.FindDirection`)
  (`KismetSystemLibrary.K2_SetTimerDelegate` (`|CreateDelegate` :!event `CreateBullet`) 2.0 true)
  (`self.CreateBullet`)
  ;[1 1 1] 에너지바 호출
  (bind _asenergybar_1 (cast `/Game/GameContents/Energybar1` (`WidgetComponent.GetUserWidgetObject` (`self.Energybarwidget`))))
  ;[1 1 1] 초기값 셋팅
  (bind _output_get (set `self.Energybar1` _asenergybar_1))
  (set `/Game/GameContents/Energybar1.Energypowerrr` (/ (`self.Energy`) (`self.NormEnergy`)) _output_get))

(event `self.ReceiveTick`
  (params (DeltaSeconds :type "Float (single-precision)"))
  (`self.K2_SetActorLocation` (+ (`self.K2_GetActorLocation`) (* (* (`self.Direction`) (`self.Speed`)) DeltaSeconds)) true true)
  (`self.FindDirection`))

(event `self.ReceiveAnyDamage`
  (params (Damage :type "Float (single-precision)") (DamageType :type "DamageType Object Reference") (InstigatedBy :type "Controller Object Reference") (DamageCauser :type "Actor Object Reference"))
  ;[1 1 1] 데미지 입력값
  (set `self.Energy` (- (`self.Energy`) Damage))
  ;[1 1 1] 에너지 잔량 입력
  (set `/Game/GameContents/Energybar1.Energypowerrr` (/ (`self.Energy`) (`self.NormEnergy`)) (`self.Energybar1`))
  ;[1 1 1] 에너지 0 이면 삭제
  (if (<= (`self.Energy`) 0.0)
    (`self.K2_DestroyActor`)))

(fn `CreateBullet`
  (`|SpawnActorFromClass` "/Game/GameContents/BP_MonsterBullet.BP_MonsterBullet_C" (`self.GetTransform`) "AlwaysSpawn" "OverrideRootScale" null null))

(fn `FindDirection`
  (bind _target (`self.Target`))
  (`/Engine/EditorBlueprintResources/StandardMacros.IsValid` _target
    (:`Is Valid`
      (set `self.Direction` (`KismetMathLibrary.Normal` (- (`self.K2_GetActorLocation` _target) (`self.K2_GetActorLocation`)))))))

(fn `UserConstructionScript`)