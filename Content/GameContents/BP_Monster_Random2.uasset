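; BP_Monster_Random2 is an enemy that homes in on BP_SnowMan and fires bullets.
; Tick sweeps it along the normalized direction to the target and updates its energy bar, while chained Delays cycle moving, stopping and spawning BP_MonsterBullet.
; Damage drains Energy and spawns damage markers; at zero it increments the player's KillCount, drops money and destroys itself.
; The win check compares constants (0 < 5), so the EndGame menu branch never runs.
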(event `self.ReceiveBeginPlay`
  (bind _returnvalue (`GameplayStatics.GetActorOfClass` "/Game/GameContents/BP_SnowMan.BP_SnowMan_C"))
  (set `self.Target` _returnvalue))

(event `self.ReceiveTick`
  (params (DeltaSeconds :type "Float (single-precision)"))
  (bind _returnvalue (+ DeltaSeconds 1.0))
  (`self.K2_SetActorLocation` (+ (`self.K2_GetActorLocation`) (* (* (`self.Direction`) (`self.Speed`)) DeltaSeconds)) true true)
  ;[1 1 1] 찾은 벡터 방향으로
  (`self.FindDirection`)
  ;[1 1 1] 에너지바 호출
  (bind _asenergybar_1 (cast `/Game/GameContents/Energybar1` (`WidgetComponent.GetUserWidgetObject` (`self.Energybarwidget`))))
  ;[1 1 1] 초기값 셋팅
  (bind _output_get (set `self.Energybar1` _asenergybar_1))
  (set `/Game/GameContents/Energybar1.Energypowerrr` (/ (`self.Energy`) (`self.NormEnergy`)) _output_get)
  ;[1 1 1] 스펀후 잠시 움직임
  (`KismetSystemLibrary.Delay` (`self.duration2`))
  ;[1 1 1] 멈췄다가 총알 발사
  (set `self.Speed` 0.0)
  (`KismetSystemLibrary.Delay` (`self.duration1`))
  (`self.CreateBullet`)
  (`KismetSystemLibrary.Delay` 0.5)
  ;[1 1 1] 딜레이 초기화
  (set `self.Speed` 100.0)
  (`KismetSystemLibrary.Delay` 2.0)
  (set `self.duration1` _returnvalue)
  (set `self.duration2` (+ _returnvalue 0.0)))

(event `self.ReceiveAnyDamage`
  (params (Damage :type "Float (single-precision)") (DamageType :type "DamageType Object Reference") (InstigatedBy :type "Controller Object Reference") (DamageCauser :type "Actor Object Reference"))
  ;[1 1 1] 데미지 입력값
  (set `self.Energy` (- (`self.Energy`) Damage))
  ;[1 1 1] 에너지 잔량 입력
  (set `/Game/GameContents/Energybar1.Energypowerrr` (/ (`self.Energy`) (`self.NormEnergy`)) (`self.Energybar1`))
  ;[1 1 1] 에너지 0 이면
  (if (<= (`self.Energy`) 0.0)
    ;[1 1 1] Monster를 KillCount+1 하고 Destroy
    (bind _asbp_snow_man (cast `/Game/GameContents/BP_SnowMan` (`GameplayStatics.GetPlayerCharacter` 0)))
    (set `/Game/GameContents/BP_SnowMan.KillCount` (+ (`/Game/GameContents/BP_SnowMan.KillCount` _asbp_snow_man) 1) _asbp_snow_man)
    ;[1 1 1] 5명을 Kill 하면 Win
    (if (< 0 5)
      (`GameplayStatics.PlaySound2D` "/Game/Title/Sounds/DiyngSound.DiyngSound" 1.0 1.0 0.0 null null)
      (`self.DropMoney`)
      (`self.K2_DestroyActor`)
      (else
        (`self.EndGame`)
        (`GameplayStatics.PlaySound2D` "/Game/Title/Sounds/CongratSound.CongratSound" 1.0 1.0 0.0 null null)))
    (else
      ;[1 1 1] 데미지 입력값이 0.5와 1에 따라 표시
      (if (<= Damage 0.5)
        (`|SpawnActorFromClass` "/Game/JWContents/BP/BP_DamagePointM.BP_DamagePointM_C" (`self.GetTransform`) "Undefined" "OverrideRootScale" null null)
        (else
          (`|SpawnActorFromClass` "/Game/JWContents/BP/BP_DamagePoint.BP_DamagePoint_C" (`self.GetTransform`) "Undefined" "OverrideRootScale" null null))))))

(event `DropMoney`
  ;[1 1 1] Money Drop Event
  (`|SpawnActorFromClass` "/Game/GameContents/Interaction/BP_Money.BP_Money_C" (`self.GetTransform`) "Undefined" "OverrideRootScale" null null))

(event `EndGame`
  ;[1 1 1] 게임을 종료하기 위한 Event
  (`GameplayStatics.SetGamePaused` true)
  (set `PlayerController.bShowMouseCursor` true (`GameplayStatics.GetPlayerController` 0))
  (bind _returnvalue (`|CreateWidget` "/Game/Title/EndMenu.EndMenu_C"))
  (`UserWidget.AddToViewport` _returnvalue 0))

(fn `CreateBullet`
  (`|SpawnActorFromClass` "/Game/GameContents/BP_MonsterBullet.BP_MonsterBullet_C" (`self.GetTransform`) "AlwaysSpawn" "OverrideRootScale" null null))

(fn `FindDirection`
  (bind _target (`self.Target`))
  (`/Engine/EditorBlueprintResources/StandardMacros.IsValid` _target
    (:`Is Valid`
      (set `self.Direction` (`KismetMathLibrary.Normal` (- (`self.K2_GetActorLocation` _target) (`self.K2_GetActorLocation`)))))))

(fn `UserConstructionScript`)