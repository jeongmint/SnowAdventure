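; BP_SnowMan is the player-controlled snowman character, which moves, looks, jumps and fires snowballs.
; Movement follows control yaw, while the Iceball function spawns a projectile and snow-steam effect at Arrow1.
; Jumping and firing each play one of two sounds at weighted random.
; AnyDamage lowers Energy, updates the widget-component energy bar as a normalized ratio, and destroys the actor at zero.
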(event `InputAxis|Vertical`
  (params (AxisValue :type "Float (single-precision)"))
  ;[1 1 1] 캐릭터 이동
  (`self.AddMovementInput` (`KismetMathLibrary.GetForwardVector` (`KismetMathLibrary.MakeRotator` 0.0 0.0 (.yaw (`self.GetControlRotation`)))) AxisValue))

(event `InputAxis|Horizon`
  (params (AxisValue :type "Float (single-precision)"))
  ;[1 1 1] 캐릭터 이동
  (`self.AddMovementInput` (`KismetMathLibrary.GetRightVector` (`KismetMathLibrary.MakeRotator` 0.0 0.0 (.yaw (`self.GetControlRotation`)))) AxisValue))

(event `InputAction|Jump`
  (params (Key :type "Key Structure"))
  ;[1 1 1] 캐릭터 이동
  (:`Pressed`
    (`self.Jump`)
    ;[1 1 1] 2가지 점프 사운드 재생
    (if (<= (`KismetMathLibrary.RandomIntegerInRange` 1 4) 3)
      (`GameplayStatics.PlaySound2D` "/Game/JWContents/Sounds/audio_1_jump.audio_1_jump" 1.0 1.0 0.0 null null)
      (else
        (`GameplayStatics.PlaySound2D` "/Game/JWContents/Sounds/audio_4_jump.audio_4_jump" 1.0 1.0 0.0 null null)))))

(event `InputAction|IceBall`
  (params (Key :type "Key Structure"))
  ;[1 1 1] 눈덩이 발사
  (:`Pressed`
    (`self.iceball`)
    ;[1 1 1] 2가지 공격 사운드 재생
    (if (<= (`KismetMathLibrary.RandomIntegerInRange` 1 4) 3)
      (`GameplayStatics.PlaySound2D` "/Game/JWContents/Sounds/audio_0_badara.audio_0_badara" 1.0 1.0 0.0 null null)
      (else
        (`GameplayStatics.PlaySound2D` "/Game/JWContents/Sounds/audio_3_snowball.audio_3_snowball" 1.0 1.0 0.0 null null)))))

(event `InputAxis|TurnRighthh`
  (params (AxisValue :type "Float (single-precision)"))
  ;[1 1 1] 화면 전환
  (`self.AddControllerYawInput` AxisValue))

(event `InputAxis|lookuphh`
  (params (AxisValue :type "Float (single-precision)"))
  ;[1 1 1] 화면 전환
  (`self.AddControllerPitchInput` AxisValue))

(event `self.ReceiveBeginPlay`
  ;[1 1 1] 에너지바 호출
  (bind _asenergybar_2 (cast `/Game/GameContents/Energybar2` (`WidgetComponent.GetUserWidgetObject` (`self.Penergywidget`))))
  ;[1 1 1] 초기값 셋팅
  (bind _output_get (set `self.As Energybar 2` _asenergybar_2))
  (set `/Game/GameContents/Energybar2.PlayerEnergy` (/ (`self.Energy`) (`self.NormEnergy`)) _output_get))

(event `self.ReceiveAnyDamage`
  (params (Damage :type "Float (single-precision)") (DamageType :type "DamageType Object Reference") (InstigatedBy :type "Controller Object Reference") (DamageCauser :type "Actor Object Reference"))
  ;[1 1 1] 데미지 입력값
  (set `self.Energy` (- (`self.Energy`) Damage))
  ;[1 1 1] 에너지 잔량 입력
  (set `/Game/GameContents/Energybar2.PlayerEnergy` (/ (`self.Energy`) (`self.NormEnergy`)) (`self.PlayerEnergyBar`))
  ;[1 1 1] 에너지 0 이면 삭제
  (if (<= (`self.Energy`) 0.0)
    (`self.K2_DestroyActor`)))

(fn `iceball`
  ;[1 1 1] 발사 효과
  (`|SpawnActorFromClass` "/Game/JWContents/BP/EmitterSnowSteam.EmitterSnowSteam_C" (`SceneComponent.K2_GetComponentToWorld` (`self.Arrow1`)) "Undefined" "OverrideRootScale" null null)
  ;[1 1 1] 눈덩이 생성 발사
  (`|SpawnActorFromClass` "/Game/GameContents/Iceball.Iceball_C" (`SceneComponent.K2_GetComponentToWorld` (`self.Arrow1`)) "Undefined" "OverrideRootScale" null null))

(fn `UserConstructionScript`)